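; B_GameHUD is the in-game HUD that draws a reticle and toggles the watch menu.
; On BeginPlay it creates the W_WatchMenu widget and caches the player character.
; Each DrawHUD call draws the reticle texture positioned from half the screen size, then polls the character's IsWatchUp flag.
; When that flag changes, it adds or removes the menu and toggles the mouse cursor, returning focus to the game viewport on close.
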(event `self.ReceiveBeginPlay`
  (bind _returnvalue (`|CreateWidget` "/Game/Blueprints/GUI/Widgets/W_WatchMenu.W_WatchMenu_C"))
  (set `self.mainGUIWidget` _returnvalue)
  (bind (_asb_character_generic _bsuccess) (`/Game/DataTypes/Functions/PlayerGets.GetIBPlayerCharacter` 0))
  (if _bsuccess
    (set `self.character` _asb_character_generic)
    (else
      (`VisualLoggerKismetLibrary.LogText` "Get Player Character Failed"))))

(event `self.ReceiveDrawHUD`
  (params (SizeX :type Integer) (SizeY :type Integer))
  (`self.DrawTexture` "/Game/Textures/reticle.reticle" (`KismetMathLibrary.Conv_IntToDouble` (/ SizeX 2)) (`KismetMathLibrary.Conv_IntToDouble` (/ SizeY 2)) 32.0 32.0 0.0 0.0 1.0 1.0)
  (`self.ShowOrHideWatch`))

(fn `ShowOrHideWatch`
  (bind _returnvalue (`GameplayStatics.GetPlayerController` 0))
  (bind _mainguiwidget (`self.mainGUIWidget`))
  (bind _iswatchvisible (`self.isWatchVisible`))
  (if (`/Game/Blueprints/GameModes/B_CharacterGeneric.isWatchUp` (`self.character`))
    (if (not _iswatchvisible)
      (set `PlayerController.bShowMouseCursor` true _returnvalue)
      (`UserWidget.AddToViewport` _mainguiwidget 0)
      (set `self.isWatchVisible` true))
    (elif _iswatchvisible
      (set `PlayerController.bShowMouseCursor` false _returnvalue)
      (`Widget.RemoveFromParent` _mainguiwidget)
      (set `self.isWatchVisible` false)
      (`WidgetBlueprintLibrary.SetFocusToGameViewport`)))
  (return))

(fn `UserConstructionScript`)