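; B_TriggerableLight is a point light that other logic can switch on and off.
; The construction script sets the PointLightComponent's visibility from IsLightOn, so the initial state shows on placement.
; TurnOn and TurnOff set that visibility, propagated to child components, and update IsLightOn to match.
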(fn `TurnOff`
  (`SceneComponent.SetVisibility` (`self.PointLightComponent`) false true)
  (set `self.isLightOn` false))

(fn `TurnOn`
  (`SceneComponent.SetVisibility` (`self.PointLightComponent`) true true)
  (set `self.isLightOn` true))

(fn `UserConstructionScript`
  (`SceneComponent.SetVisibility` (`self.PointLightComponent`) (`self.isLightOn`) true))