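; Modular tile actor that assembles a floor, ceiling, walls, doors and corner pieces in its construction script.
; Walls and WallIsDoor bitmasks pick a wall or door for each of four sides, rotated in 90-degree steps plus per-piece orientation overrides.
; Adjacent-side bit pairs decide inside corners, and outside corners where both sides are open, which are skipped when IsRoom is set.
; Each piece is added as a static mesh component.
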(fn `UserConstructionScript`
  (locals (NewLocalVar_0 :type "StaticMeshComponent Object Reference"))
  (bind _returnvalue (`|BitmaskLiteral` 3))
  (bind _returnvalue_2 (`|BitmaskLiteral` 6))
  (bind _returnvalue_3 (`|BitmaskLiteral` 12))
  (bind _returnvalue_4 (`|BitmaskLiteral` 9))
  (bind _returnvalue_5 (`|BitmaskLiteral` 3))
  (bind _returnvalue_6 (`|BitmaskLiteral` 6))
  (bind _returnvalue_7 (`|BitmaskLiteral` 12))
  (bind _returnvalue_8 (`|BitmaskLiteral` 9))
  (bind (_floor _ceiling _wall _door _corner_inside _corner_outside) (`self.MeshMegaGet`))
  (bind _walls (`self.Walls`))
  (bind _outsidecorneroverride (`self.outsideCornerOverride`))
  (bind _walls_2 (`self.Walls`))
  (bind _wallisdoor (`self.WallIsDoor`))
  (bind _insidecorneroverride (`self.insideCornerOverride`))
  (`self.AddAndSetMesh` _floor)
  (`self.AddAndSetMesh` _ceiling)
  (for _index (range 4)
    (bind _returnvalue_9 (`KismetMathLibrary.FTrunc` (`KismetMathLibrary.MultiplyMultiply_FloatFloat` 2.0 (`KismetMathLibrary.Conv_IntToDouble` _index))))
    (if (`KismetMathLibrary.Conv_IntToBool` (`KismetMathLibrary.And_IntInt` (`self.Walls`) _returnvalue_9))
      (if (`KismetMathLibrary.Conv_IntToBool` (`KismetMathLibrary.And_IntInt` (`self.WallIsDoor`) _returnvalue_9))
        (`self.AddAndSetMesh` _door (+ _index (`self.doorOverride`)))
        (else
          (`self.AddAndSetMesh` _wall (+ _index (`self.wallOverride`)))))))
  (if (or (== (`KismetMathLibrary.And_IntInt` _walls_2 _returnvalue_5) _returnvalue_5) (== (`KismetMathLibrary.And_IntInt` _wallisdoor _returnvalue) _returnvalue))
    (`self.AddAndSetMesh` _corner_inside (+ _insidecorneroverride 0)))
  (if (or (== (`KismetMathLibrary.And_IntInt` _walls_2 _returnvalue_6) _returnvalue_6) (== (`KismetMathLibrary.And_IntInt` _wallisdoor _returnvalue_2) _returnvalue_2))
    (`self.AddAndSetMesh` _corner_inside (+ _insidecorneroverride 1)))
  (if (or (== (`KismetMathLibrary.And_IntInt` _walls_2 _returnvalue_7) _returnvalue_7) (== (`KismetMathLibrary.And_IntInt` _wallisdoor _returnvalue_3) _returnvalue_3))
    (`self.AddAndSetMesh` _corner_inside (+ _insidecorneroverride 2)))
  (if (or (== (`KismetMathLibrary.And_IntInt` _walls_2 _returnvalue_8) _returnvalue_8) (== (`KismetMathLibrary.And_IntInt` _wallisdoor _returnvalue_4) _returnvalue_4))
    (`self.AddAndSetMesh` _corner_inside (+ _insidecorneroverride 3)))
  (if (not (`self.IsRoom`))
    (if (== (`KismetMathLibrary.And_IntInt` _walls (`|BitmaskLiteral` 3)) 0)
      (`self.AddAndSetMesh` _corner_outside (+ _outsidecorneroverride 0)))
    (if (== (`KismetMathLibrary.And_IntInt` _walls (`|BitmaskLiteral` 6)) 0)
      (`self.AddAndSetMesh` _corner_outside (+ _outsidecorneroverride 1)))
    (if (== (`KismetMathLibrary.And_IntInt` _walls (`|BitmaskLiteral` 12)) 0)
      (`self.AddAndSetMesh` _corner_outside (+ _outsidecorneroverride 2)))
    (if (== (`KismetMathLibrary.And_IntInt` _walls (`|BitmaskLiteral` 9)) 0)
      (`self.AddAndSetMesh` _corner_outside (+ _outsidecorneroverride 3)))))