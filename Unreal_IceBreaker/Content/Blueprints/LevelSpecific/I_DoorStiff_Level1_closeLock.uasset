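; Level 1 stiff door Blueprint variant that sets its lock flag to false and its door state to an enumerator value when play begins.
; On interact, a door in the Open state switches to another state and plays the OpenDoorSlowly timeline in reverse from the end.
; Other states have no interaction response here, and the forward play of that timeline is never executed.
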(event `self.ReceiveBeginPlay`
  (set `self.isLocked` false)
  (set `self.edoorstate` 0))

(event `/Game/Blueprints/Interactable/Interactable.OnInteract`
  (params (WhoCalled :type "/Game/Blueprints/GameModes/B_CharacterGeneric Object Reference"))
  (switch `/Game/Blueprints/DataTypes/Enums/DoorState` (`self.edoorstate`)
    (:`NewEnumerator2`
      (set `self.edoorstate` 0)
      (`TimelineComponent.ReverseFromEnd` (`self.Open Door Slowly`)))))

(fn `UserConstructionScript`
  (`parent.UserConstructionScript`))