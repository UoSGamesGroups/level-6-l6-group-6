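; Interactable utility door built from a resizable cube that swings between closed and open on interact.
; The construction script scales the cube from the TopCorner component's relative location and poses the hinge open if the door starts Open.
; The Slow Door Open graph plays or reverses a timeline that lerps the hinge transform.
; A four-state DoorState ignores interaction while the door is moving.
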(event `/Game/Blueprints/Interactable/Interactable.OnInteract`
  (params (WhoCalled :type "/Game/Blueprints/B_CharacterGeneric Object Reference"))
  (switch `/Game/Blueprints/Interactable/DoorState` (`self.doorState`)
    (:`NewEnumerator0`
      (set `self.doorState` "NewEnumerator1")
      (bind (_direction _open_amount) (`Timeline|Open Door Slowly` :!label _label)
        (:`Update`
          (`SceneComponent.K2_SetRelativeTransform` (`self.Door Hinge`) (`KismetMathLibrary.TLerp` (`self.ClosedRotation`) (`self.OpenRotation`) _open_amount) false false))
        (:`Finished`
          (switch `/Game/Blueprints/Interactable/DoorState` (`self.doorState`)
            (:`NewEnumerator1`
              (set `self.doorState` "NewEnumerator2"))
            (:`NewEnumerator3`
              (set `self.doorState` "NewEnumerator0"))))))
    (:`NewEnumerator2`
      (set `self.doorState` "NewEnumerator3")
      (goto _label :!via `ReverseFromEnd`))))

(fn `UserConstructionScript`
  (bind _cubetransform (`self.CubeTransform`))
  (`parent.UserConstructionScript`)
  (`SceneComponent.K2_SetWorldTransform` _cubetransform (`KismetMathLibrary.MakeTransform` (.location (`SceneComponent.K2_GetComponentToWorld` _cubetransform)) (.rotation (`SceneComponent.K2_GetComponentToWorld` _cubetransform)) (/ (.location (`SceneComponent.GetRelativeTransform` (`self.Top Corner`))) 100)) false false)
  (if (`|EnumEquality` (`self.doorState`) "NewEnumerator2")
    (`SceneComponent.K2_SetRelativeTransform` (`self.Door Hinge`) (`self.OpenRotation`) false false)))