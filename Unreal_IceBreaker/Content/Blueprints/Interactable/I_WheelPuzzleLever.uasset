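; Interactable lever for a wheel puzzle that can be pulled while not activated and reports to its parent puzzle.
; OnInteract sets IsActivated and plays a timeline that lerps the actor between resting and activated rotations.
; When the timeline finishes, it passes LeverNumber to LeverHit on PuzzleParent, which is assigned through SetPuzzleParent.
; Reset reverses the timeline, and nothing in this Blueprint clears IsActivated.
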(event `self.OnInteract`
  (if (not (`self.isActivated`))
    (set `self.isActivated` true)
    (bind (_direction _lerpmask) (`Timeline|ActivateAnimation` :!label _label)
      (:`Update`
        (`self.K2_SetActorRotation` (`KismetMathLibrary.RLerp` (`self.restingRotation`) (`self.activatedRotation`) _lerpmask))
        (set `self.isActivated` true))
      (:`Finished`
        (`/Game/Blueprints/Prototype/B_PTTP_WheelPuzzle.Lever Hit` (`self.puzzleParent`) (`self.leverNumber`))))))

(event `Reset`
  (goto _label :!via `Reverse`))

(fn `SetPuzzleParent`
  (params (PuzzleParent :type "/Game/Blueprints/Prototype/B_PTTP_WheelPuzzle Object Reference"))
  (set `self.puzzleParent` PuzzleParent))

(fn `UserConstructionScript`
  (`parent.UserConstructionScript`))