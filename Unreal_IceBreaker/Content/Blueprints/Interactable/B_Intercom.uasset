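; B_Intercom is an interactable intercom actor that flashes a point light and triggers a buzz in a repeating cycle from BeginPlay.
; A looping timer fires BuzzTick every LightFlashTime, which shows the light, spawns a sound at the world origin, then hides the light halfway through the interval.
; The construction script starts the light hidden, and TriggerCallStart is an empty stub, so nothing here stops the buzzing.
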(event `self.ReceiveBeginPlay`
  (`self.LightFlashAndBuzz`))

(event `LightFlashAndBuzz`
  ;[1 1 1] Toggle on wait off wait
  (`KismetSystemLibrary.K2_SetTimerDelegate` (delegate `BuzzTick`) (`self.lightFlashTime`) true))

(event `BuzzTick`
  (bind _pointlight (`self.PointLight`))
  (bind _returnvalue (/ (`self.lightFlashTime`) 2.0))
  ;[1 1 1] Toggle on wait off wait
  (`SceneComponent.SetVisibility` _pointlight true false)
  (`GameplayStatics.SpawnSoundAtLocation` null)
  (`KismetSystemLibrary.Delay` _returnvalue)
  (`SceneComponent.SetVisibility` _pointlight false false)
  (`KismetSystemLibrary.Delay` _returnvalue))

(fn `TriggerCallStart`)

(fn `UserConstructionScript`
  (`parent.UserConstructionScript`)
  (`SceneComponent.SetVisibility` (`self.PointLight`) false false))