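; B_Lever is an interactable lever that switches on one way, and only once it has been unlocked.
; On interact, an unlocked lever plays a timeline blending the model from its construction-time idle transform to EnabledTransform, then sets IsEnabled.
; A locked lever plays a Jiggle timeline along the same blend instead.
; UnlockLever clears the lock, and GetIsEnabled exposes the state.
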(event `self.OnInteract`
  (params (WhoCalled :type "/Game/Blueprints/GameModes/B_CharacterGeneric Object Reference"))
  (bind _levermodel (`self.LeverModel`))
  (if (`self.isEnabled`)
    _
    (elif (`self.isUnlocked`)
      (bind (_direction _alpha) (`Timeline|Enable` :!via `PlayFromStart`)
        (:`Update`
          (`SceneComponent.K2_SetRelativeTransform` _levermodel (`KismetMathLibrary.TLerp` (`self.idleTransform`) (`self.enabledTransform`) _alpha) false false))
        (:`Finished`
          (set `self.isEnabled` true)))
      (else
        (bind (_direction_2 _jiggle) (`Timeline|Jiggle` :!via `PlayFromStart`)
          (:`Update`
            (`SceneComponent.K2_SetRelativeTransform` _levermodel (`KismetMathLibrary.TLerp` (`self.idleTransform`) (`self.enabledTransform`) _jiggle) false false)))))))

(event `UnlockLever`
  (set `self.isUnlocked` true))

(fn `GetIsEnabled`
  (returns (isEnabled :type Boolean))
  (return (`self.isEnabled`)))

(fn `UserConstructionScript`
  (`parent.UserConstructionScript`)
  (set `self.idleTransform` (`SceneComponent.GetRelativeTransform` (`self.LeverModel`))))