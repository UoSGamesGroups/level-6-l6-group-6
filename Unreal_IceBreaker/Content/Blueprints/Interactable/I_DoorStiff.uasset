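; Interactable stiff door that slowly opens or closes when interacted with, ignoring interaction while it is moving.
; OnInteract switches on DoorState and calls Open or Close in the Slow Door Open graph.
; That graph plays or reverses the OpenDoorSlowly timeline, lerping the door mesh's relative transform between closed and open, then settles the state when the timeline finishes.
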(event `/Game/Blueprints/Interactable/Interactable.OnInteract`
  (switch `/Game/Blueprints/Interactable/DoorState` (`self.doorState`)
    (:`NewEnumerator0`
      (set `self.doorState` "NewEnumerator1")
      (bind (_direction _open_amount) (`Timeline|Open Door Slowly` :!label _label)
        (:`Update`
          (`SceneComponent.K2_SetRelativeTransform` (`self.Door Mesh`) (`KismetMathLibrary.TLerp` (`self.ClosedRotation`) (`self.OpenRotation`) _open_amount) false false))
        (:`Finished`
          (switch `/Game/Blueprints/Interactable/DoorState` (`self.doorState`)
            (:`NewEnumerator1`
              (set `self.doorState` "NewEnumerator2"))
            (:`NewEnumerator3`
              (set `self.doorState` "NewEnumerator0"))))))
    (:`NewEnumerator2`
      (set `self.doorState` "NewEnumerator3")
      (goto _label :!via `ReverseFromEnd`))))

(fn `UserConstructionScript`
  (`parent.UserConstructionScript`))