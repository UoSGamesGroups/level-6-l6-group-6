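; AI character that switches into an aggro state on seeing a B_CharacterGeneric pawn and manipulates nearby lights.
; PawnSensing sightings set the state and refresh LocalLights by sphere overlap; a retriggerable delay drops aggro once sightings stop, and Tick swaps idle and pursuit vision angles.
; BeginPlay hides nearby PointLights.
; LightsOff and LightsOn toggle cached B_PointLight_Coll lights but are uncalled here, and a timed light-blink chain is disconnected.
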(event `self.ReceiveBeginPlay`
  (bind _outactors (`KismetSystemLibrary.SphereOverlapActors_NEW` (`self.K2_GetActorLocation`) (`self.LightCheckRadius`) (`|MakeArray` "ObjectTypeQuery2" :!type "EObjectTypeQuery Enum") "/Script/Engine.PointLight"))
  (set `self.LocalLights` _outactors)
  (for _array_element (`self.LocalLights`)
    (`self.SetActorHiddenInGame` _array_element true)))

(event `self.ReceiveTick`
  (params (DeltaSeconds :type "Float (single-precision)"))
  (bind _pawnsensing (`self.PawnSensing`))
  (if (`|EnumEquality` (`self.AIAggroState`) "NewEnumerator1")
    (`PawnSensingComponent.SetPeripheralVisionAngle` _pawnsensing (`self.FOVPersue`))
    (else
      (`PawnSensingComponent.SetPeripheralVisionAngle` _pawnsensing (`self.FOVIdle`)))))

(event `self.PawnSensing.OnSeePawn`
  (params (Pawn :type "Pawn Object Reference"))
  (cast `/Game/Blueprints/GameModes/B_CharacterGeneric` Pawn)
  (set `self.AIAggroState` "NewEnumerator1")
  (`self.FindLights`)
  (`KismetSystemLibrary.RetriggerableDelay` (* (`PawnSensingComponent.SensingInterval` (`self.PawnSensing`)) 2.0))
  (set `self.AIAggroState` "NewEnumerator0"))

(fn `FindLights`
  (bind _outactors (`KismetSystemLibrary.SphereOverlapActors_NEW` (`self.K2_GetActorLocation`) (`self.LightCheckRadius`) (`|MakeArray` "ObjectTypeQuery2" :!type "EObjectTypeQuery Enum") "/Game/Blueprints/B_PointLight_Coll.B_PointLight_Coll_C"))
  (set `self.LocalLights` _outactors))

(fn `LightsOff`
  (for _array_element (`self.LocalLights`)
    (bind _asb_point_light_coll (cast `/Game/Blueprints/B_PointLight_Coll` _array_element))
    (`/Game/Blueprints/B_PointLight_Coll.SetIsOn` _asb_point_light_coll false)))

(fn `LightsOn`
  (for _array_element (`self.LocalLights`)
    (bind _asb_point_light_coll (cast `/Game/Blueprints/B_PointLight_Coll` _array_element))
    (`/Game/Blueprints/B_PointLight_Coll.SetIsOn` _asb_point_light_coll true)))

(fn `UserConstructionScript`
  (set `self.FOVIdle` (`PawnSensingComponent.GetPeripheralVisionAngle` (`self.PawnSensing`))))