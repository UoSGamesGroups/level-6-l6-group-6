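; Blueprint function collection that provides per-tick movement logic for two AI types, Scampers and Sprinters.
; TickScamper teleports a Scamper in blink-sized steps toward player 0, yawed to face them, until within arrival distance.
; TickSprinter uses simple move nodes to chase the player in one aggro state, otherwise walking a passed-in waypoint array and advancing its index on arrival.
; An older controller-based teleport remains unconnected.
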(fn `TickScamper`
  (params (TargetScamper :type "/Game/Blueprints/AI/B_PTTP_AIScamper Object Reference"))
  (bind _returnvalue (`Actor.K2_GetActorLocation` TargetScamper))
  (bind _returnvalue_2 (`Actor.K2_GetActorLocation` (`GameplayStatics.GetPlayerCharacter` null)))
  ;[1 1 1] if scamper isnt at player yet
  (if (> (`Actor.GetDistanceTo` (`GameplayStatics.GetPlayerCharacter` null) TargetScamper) (`/Game/Blueprints/AI/B_PTTP_AIScamper.ArrivalDistance` TargetScamper))
    (`Actor.K2_TeleportTo` TargetScamper (+ _returnvalue (* (`KismetMathLibrary.GetDirectionVector` _returnvalue _returnvalue_2) (`/Game/Blueprints/AI/B_PTTP_AIScamper.blinkDistance` TargetScamper))) (`KismetMathLibrary.MakeRotator` 0.0 0.0 (.yaw (`KismetMathLibrary.FindLookAtRotation` _returnvalue _returnvalue_2))))))

(fn `TickSprinter`
  (params (SprinterInLevel :type "/Game/Blueprints/AI/B_PTTP_AISprinter Object Reference") (TargetArray :type "Array of TargetPoint Object Reference (by ref)"))
  (bind _item (`KismetArrayLibrary.Array_Get` TargetArray (`/Game/Blueprints/AI/B_PTTP_AISprinter.CurrentTarget` SprinterInLevel)))
  (if (`|EnumEquality` (`/Game/Blueprints/AI/B_PTTP_AISprinter.AIAggroState` SprinterInLevel) "NewEnumerator1")
    ;[1 1 1] FollowPlayer
    (`NavigationSystem.SimpleMoveToActor` (`Pawn.GetController` SprinterInLevel) (`GameplayStatics.GetPlayerCharacter` null))
    (else
      ;[1 1 1] MoveToWaypoint
      (`NavigationSystem.SimpleMoveToLocation` (`Pawn.GetController` SprinterInLevel) (`Actor.K2_GetActorLocation` _item))
      ;[1 1 1] Has the AI arrived at the target
      (if (<= (`Actor.GetDistanceTo` SprinterInLevel _item) (`/Game/Blueprints/AI/B_PTTP_AISprinter.ArrivalDistance` SprinterInLevel))
        ;[1 1 1] Set the AI to go to the next target
        (bind _result (`/Engine/EditorBlueprintResources/StandardMacros.IncrementInt` (`/Game/Blueprints/AI/B_PTTP_AISprinter.CurrentTarget` SprinterInLevel))
          (:`  `
            (if (> _result (`KismetArrayLibrary.Array_Length` TargetArray))
              (set `/Game/Blueprints/AI/B_PTTP_AISprinter.CurrentTarget` 0 SprinterInLevel))))))))