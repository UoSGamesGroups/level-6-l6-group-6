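; B_AISprinter is an AI Blueprint that drives its aggro state from pawn sight.
; Seeing a generic character while player 0 is not hiding sets an alerted state.
; A retriggerable delay holds that state until sightings lapse, then switches to a follow-up state and refills the pace counter.
; Tick restores the default state once that counter runs out; movement and pace countdown are not handled in this graph.
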(event `self.ReceiveTick`
  (params (DeltaSeconds :type "Float (single-precision)"))
  (if (and (`|EnumEquality` (`self.AIAggroState`) "NewEnumerator2") (<= (`self.numPaces`) 0))
    (set `self.AIAggroState` "NewEnumerator0")))

(event `self.PawnSensing.OnSeePawn`
  (params (Pawn :type "Pawn Object Reference"))
  (bind _asb_character_generic (`/Game/DataTypes/Functions/PlayerGets.GetIBPlayerCharacter` 0))
  (if (not (`/Game/Blueprints/GameModes/B_CharacterGeneric.isHiding` _asb_character_generic))
    (cast `/Game/Blueprints/GameModes/B_CharacterGeneric` Pawn)
    (set `self.AIAggroState` "NewEnumerator1")
    (`KismetSystemLibrary.RetriggerableDelay` 3.0)
    (set `self.AIAggroState` "NewEnumerator2")
    (set `self.numPaces` (`self.maxNumPaces`))))

(fn `UserConstructionScript`)