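; A player character Blueprint that handles camera look input, with movement only partly built.
; The LookUp and Turn axis events feed controller pitch and yaw input directly.
; MoveForward and MoveRight events are empty, and the nodes for building a 2D move vector and adding movement input are left disconnected, so neither axis moves the character.
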(event `InputAxis|MoveRight`
  (params (AxisValue :type "Float (single-precision)"))
  ;[1 1 1] Getting movement input
)

(event `InputAxis|MoveForward`
  (params (AxisValue :type "Float (single-precision)"))
  ;[1 1 1] Getting movement input
)

(event `InputAxis|LookUp`
  (params (AxisValue :type "Float (single-precision)"))
  ;[1 1 1] Look
  (`self.AddControllerPitchInput` AxisValue))

(event `InputAction|Run`
  (params (Key :type "Key Structure" :default "AnyKey")))

(event `InputAxis|Turn`
  (params (AxisValue :type "Float (single-precision)"))
  ;[1 1 1] Look
  (`self.AddControllerYawInput` AxisValue))

(fn `UserConstructionScript`)