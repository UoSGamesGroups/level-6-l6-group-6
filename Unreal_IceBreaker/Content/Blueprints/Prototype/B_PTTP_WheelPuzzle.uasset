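; Prototype three-lever combination puzzle that moves two ceiling pieces and a floor piece.
; Construction retracts the pieces and gives each child lever its number and a parent reference.
; Lever hits build a three-digit code as decimal digits, checked against ValidCombination, with per-lever timelines lerping pieces to extended transforms.
; A wrong code clears the combination, resets the levers and retracts all pieces.
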(event `self.ReceiveBeginPlay`)

(event `Lever Hit`
  (params (leverNumber :type Integer))
  (bind _currentcombination (`self.currentCombination`))
  (bind _output_get (set `self.currentCombination` (* (`self.currentCombination`) 10)))
  (set `self.currentCombination` (+ _output_get leverNumber 1))
  (if (and (>= _currentcombination 100) (< _currentcombination 1000))
    (if (== (`self.currentCombination`) (`self.validCombination`))
      (if (not (`self.isSolved`)) :!label _label
        ;[1 1 1] Lerping to activated position
        (`self.BreakOnLeverNumber` leverNumber
          (:`0`
            (bind (_direction _lerpalpha) (`Timeline|Extend_L` :!via `PlayFromStart`)
              (:`Update`
                (`SceneComponent.K2_SetRelativeTransform` (`self.CeilingPiece_L`) (`KismetMathLibrary.TLerp` (`self.leftRetracted`) (`self.leftExtended`) _lerpalpha) false false))))
          (:`1`
            (bind (_direction_2 _newtrack_1) (`Timeline|Extend_C` :!via `PlayFromStart`)
              (:`Update`
                (`SceneComponent.K2_SetRelativeTransform` (`self.FloorPiece`) (`KismetMathLibrary.TLerp` (`self.floorRetracted`) (`self.floorExtended`) _newtrack_1) false false))))
          (:`2`
            (bind (_direction_3 _newtrack_2) (`Timeline|Extend_R` :!via `PlayFromStart`)
              (:`Update`
                (`SceneComponent.K2_SetRelativeTransform` (`self.CeilingPiece_R`) (`KismetMathLibrary.TLerp` (`self.rightRetracted`) (`self.rightExtended`) _newtrack_2) false false))))))
      (else
        (`self.ResetPuzzle`)))
    (else
      (goto _label))))

(event `ResetPuzzle`
  (set `self.currentCombination` 0)
  (`self.ResetLevers`)
  ;[1 1 1] Retract Puzzle
  (bind (_direction _lerpalpha) (`Timeline|Retract` :!via `PlayFromStart`)
    (:`Update`
      (`SceneComponent.K2_SetRelativeTransform` (`self.CeilingPiece_L`) (`KismetMathLibrary.TLerp` (`self.leftExtended`) (`self.leftRetracted`) _lerpalpha) false false)
      (`SceneComponent.K2_SetRelativeTransform` (`self.FloorPiece`) (`KismetMathLibrary.TLerp` (`self.floorExtended`) (`self.floorRetracted`) _lerpalpha) false false)
      (`SceneComponent.K2_SetRelativeTransform` (`self.CeilingPiece_R`) (`KismetMathLibrary.TLerp` (`self.rightExtended`) (`self.rightRetracted`) _lerpalpha) false false))))

(fn `ResetLevers`
  (returns (worked :type Boolean))
  (bind _asi_wheel_puzzle_lever (cast `/Game/Blueprints/Interactable/I_WheelPuzzleLever` (`ChildActorComponent.ChildActor` (`self.Lever_0`)))
    (:`then`
      (`/Game/Blueprints/Interactable/I_WheelPuzzleLever.Reset` _asi_wheel_puzzle_lever)
      (bind _asi_wheel_puzzle_lever_2 (cast `/Game/Blueprints/Interactable/I_WheelPuzzleLever` (`ChildActorComponent.ChildActor` (`self.Lever_1`)))
        (:`then`
          (`/Game/Blueprints/Interactable/I_WheelPuzzleLever.Reset` _asi_wheel_puzzle_lever_2)
          (bind _asi_wheel_puzzle_lever_3 (cast `/Game/Blueprints/Interactable/I_WheelPuzzleLever` (`ChildActorComponent.ChildActor` (`self.Lever_2`)))
            (:`then`
              (`/Game/Blueprints/Interactable/I_WheelPuzzleLever.Reset` _asi_wheel_puzzle_lever_3)
              (return true))
            (:`CastFailed`
              _)))
        (:`CastFailed`
          _)))
    (:`CastFailed`
      _))
  (return false))

(fn `SetLeverN`
  (params (ChildLever :type "ChildActorComponent Object Reference") (leverNumber :type Integer))
  (bind _asi_wheel_puzzle_lever (`self.LeverActorCast` ChildLever)
    (:`then`
      (set `/Game/Blueprints/Interactable/I_WheelPuzzleLever.leverNumber` leverNumber _asi_wheel_puzzle_lever)
      (set `/Game/Blueprints/Interactable/I_WheelPuzzleLever.puzzleParent` self _asi_wheel_puzzle_lever))))

(fn `UserConstructionScript`
  (`SceneComponent.K2_SetRelativeTransform` (`self.FloorPiece`) (`self.floorRetracted`) false false)
  (`SceneComponent.K2_SetRelativeTransform` (`self.CeilingPiece_R`) (`self.rightRetracted`) false false)
  (`SceneComponent.K2_SetRelativeTransform` (`self.CeilingPiece_L`) (`self.leftRetracted`) false false)
  (`self.SetLeverN` (`self.Lever_0`))
  (`self.SetLeverN` (`self.Lever_1`) 1)
  (`self.SetLeverN` (`self.Lever_2`) 2))