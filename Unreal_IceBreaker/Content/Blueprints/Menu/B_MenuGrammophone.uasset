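; Menu gramophone that takes a "Play"-tagged B_Pickupable record onto its spindle and drops it off when interacted with.
; Overlapping GetRecordVolume makes the player release the record, disables its physics and collision, then a timeline lerps it to the spindle.
; OnInteract moves it along a spline, then restores physics and collision.
; Construction script caches the spindle transform and sets the spline's endpoint from RemovedPile.
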(event `self.GetRecordVolume.OnComponentBeginOverlap`
  (params (OverlappedComponent :type "PrimitiveComponent Object Reference") (OtherActor :type "Actor Object Reference") (OtherComp :type "PrimitiveComponent Object Reference") (OtherBodyIndex :type Integer) (bFromSweep :type Boolean) (SweepResult :type "HitResult Structure (by ref)"))
  (bind _staticmesh (`/Game/Blueprints/Puzzles/BilgePump/B_Pickupable.StaticMesh` (`self.recordRef`)))
  ;[1 1 1] Was it a pickupable that overlapped
  (bind _asb_pickupable (cast `/Game/Blueprints/Puzzles/BilgePump/B_Pickupable` OtherActor))
  (if (`self.ActorHasTag` _asb_pickupable "Play")
    ;[1 1 1] Drop the record
    (set `self.recordRef` _asb_pickupable)
    (bind (_asb_character_generic _bsuccess) (`/Game/Blueprints/DataTypes/Functions/PlayerGets.GetIBPlayerCharacter` 0))
    (if _bsuccess
      (`/Game/Blueprints/GameModes/B_CharacterGeneric.DropPhysObj` _asb_character_generic)
      (`PrimitiveComponent.SetSimulatePhysics` _staticmesh false)
      (`PrimitiveComponent.SetCollisionEnabled` _staticmesh "NoCollision")
      ;[1 1 1] Move record onto spindle
      (set `self.placeRecordStartTransform` (`SceneComponent.K2_GetComponentToWorld` (`/Game/Blueprints/Puzzles/BilgePump/B_Pickupable.StaticMesh` (`self.recordRef`))))
      (bind (_direction _lerpalpha) (`Timeline|PlaceRecordTimeline` :!via `PlayFromStart`)
        (:`Update`
          (`SceneComponent.K2_SetWorldTransform` (`/Game/Blueprints/Puzzles/BilgePump/B_Pickupable.StaticMesh` (`self.recordRef`)) (`KismetMathLibrary.TLerp` (`self.placeRecordStartTransform`) (`self.spindleTrans`) _lerpalpha) false false))))))

(event `self.OnInteract`
  (params (WhoCalled :type "/Game/Blueprints/GameModes/B_CharacterGeneric Object Reference"))
  (bind _staticmesh (`/Game/Blueprints/Puzzles/BilgePump/B_Pickupable.StaticMesh` (`self.recordRef`)))
  (`/Engine/EditorBlueprintResources/StandardMacros.IsValid` (`self.recordRef`)
    (:`Is Valid`
      (bind (_direction _lerpalpha) (`Timeline|DropRecordTimeline` :!via `PlayFromStart`)
        (:`Update`
          (`SceneComponent.K2_SetWorldTransform` (`/Game/Blueprints/Puzzles/BilgePump/B_Pickupable.StaticMesh` (`self.recordRef`)) (`SplineComponent.GetTransformAtTime` (`self.Spline`) _lerpalpha "World" false false) false false))
        (:`Finished`
          (`PrimitiveComponent.SetSimulatePhysics` _staticmesh true)
          (`PrimitiveComponent.SetCollisionEnabled` _staticmesh "QueryAndPhysics"))))))

(fn `UserConstructionScript`
  (bind _spline (`self.Spline`))
  ;[1 1 1] Set spindle pos from arrow helper
  (set `self.spindleTrans` (`SceneComponent.K2_GetComponentToWorld` (`self.RecordSpindle`)))
  ;[1 1 1] Set last position of record drop spline to drop point
  (`SplineComponent.SetLocationAtSplinePoint` _spline (- (`SplineComponent.GetNumberOfSplinePoints` _spline) 1) (- (.location (`self.RemovedPile`)) (`SceneComponent.RelativeLocation` _spline)) "Local" true))