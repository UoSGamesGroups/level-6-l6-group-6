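; Generic player character with walk and look input, a hold-to-run speed switch, interaction and a toggleable watch.
; Tick refreshes the move and look flags that gate input; raising the watch blocks looking, while SetCanMove leaves its hiding-and-watch check unconnected.
; Interact line-traces from the camera and calls OnInteract on any hit Interactable.
; A surface-based footstep sound trace is present but never runs.
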(event `self.ReceiveTick`
  (params (DeltaSeconds :type "Float (single-precision)"))
  (set `self.canMove` (`KismetMathLibrary.BooleanNOR` (`self.isHiding`) (`self.isWatchUp`)))
  (set `self.canLook` (not (`self.isWatchUp`))))

(event `InputAxis|MoveForward`
  (params (AxisValue :type "Float (single-precision)"))
  ;[1 1 1] Move
  (if (`self.canMove`)
    (`self.AddMovementInput` (`self.GetActorForwardVector`) AxisValue)))

(event `InputAxis|Turn`
  (params (AxisValue :type "Float (single-precision)"))
  ;[1 1 1] Look
  (if (`self.canLook`)
    (`self.AddControllerYawInput` AxisValue)))

(event `InputAxis|MoveRight`
  (params (AxisValue :type "Float (single-precision)"))
  ;[1 1 1] Move
  (if (`self.canMove`)
    (`self.AddMovementInput` (`self.GetActorRightVector`) AxisValue)))

(event `InputAxis|LookUp`
  (params (AxisValue :type "Float (single-precision)"))
  ;[1 1 1] Look
  (if (`self.canLook`)
    (`self.AddControllerPitchInput` AxisValue)))

(event `InputAction|Run`
  (params (Key :type "Key Structure" :default "AnyKey"))
  ;[1 1 1] Set Run
  (:`Pressed`
    (set `CharacterMovementComponent.MaxWalkSpeed` (`self.runSpeed`) (`self.CharacterMovement`)))
  (:`Released`
    (set `CharacterMovementComponent.MaxWalkSpeed` (`self.walkSpeed`) (`self.CharacterMovement`))))

(event `InputAction|Interact`
  (params (Key :type "Key Structure" :default "AnyKey"))
  (bind _returnvalue (`GameplayStatics.GetPlayerCameraManager` 0))
  (bind _returnvalue_2 (`self.K2_GetActorLocation` _returnvalue))
  (:`Pressed`
    (bind _outhit (`KismetSystemLibrary.LineTraceSingle` _returnvalue_2 (+ _returnvalue_2 (* (`self.GetActorForwardVector` _returnvalue) (`self.interactDistance`))) "TraceTypeQuery1"))
    (bind _asinteractable (cast `/Game/Blueprints/Interactable/Interactable` (`.HitActor` (`GameplayStatics.BreakHitResult` _outhit))))
    (`/Game/Blueprints/Interactable/Interactable.OnInteract` _asinteractable self)))

(event `InputAction|Watch`
  (params (Key :type "Key Structure" :default "AnyKey"))
  (:`Pressed`
    (bind _isa (`/Engine/EditorBlueprintResources/StandardMacros.FlipFlop`)
      (:`A`
        _)
      (:`B`
        _))
    (set `self.isWatchUp` _isa)))

(fn `UserConstructionScript`
  (set `CharacterMovementComponent.MaxWalkSpeed` (`self.walkSpeed`) (`self.CharacterMovement`)))