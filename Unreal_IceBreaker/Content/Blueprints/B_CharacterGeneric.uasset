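; B_CharacterGeneric is a player character with axis-driven movement and look, a hold-to-run speed switch, interaction and a raisable watch.
; Interact line-traces forward from the camera manager on the Visibility channel and calls OnInteract on a hit Interactable.
; Holding Watch plays a timeline that lerps Watch01 between start and end transforms, reversing on release.
; The construction script applies walk speed and the watch's start transform.
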(event `InputAxis|MoveForward`
  (params (AxisValue :type "Float (single-precision)"))
  ;[1 1 1] Move
  (`self.AddMovementInput` (`self.GetActorForwardVector`) AxisValue))

(event `InputAxis|Turn`
  (params (AxisValue :type "Float (single-precision)"))
  ;[1 1 1] Look
  (`self.AddControllerYawInput` AxisValue))

(event `InputAxis|MoveRight`
  (params (AxisValue :type "Float (single-precision)"))
  ;[1 1 1] Move
  (`self.AddMovementInput` (`self.GetActorRightVector`) AxisValue))

(event `InputAxis|LookUp`
  (params (AxisValue :type "Float (single-precision)"))
  ;[1 1 1] Look
  (`self.AddControllerPitchInput` AxisValue))

(event `InputAction|Run`
  (params (Key :type "Key Structure" :default "AnyKey"))
  ;[1 1 1] Set Run
  (:`Pressed`
    (set `CharacterMovementComponent.MaxWalkSpeed` (`self.runSpeed`) (`self.CharacterMovement`)))
  (:`Released`
    (set `CharacterMovementComponent.MaxWalkSpeed` (`self.walkSpeed`) (`self.CharacterMovement`))))

(event `InputAction|Interact`
  (params (Key :type "Key Structure" :default "AnyKey"))
  (bind _returnvalue (`GameplayStatics.GetPlayerCameraManager` 0))
  (bind _returnvalue_2 (`self.K2_GetActorLocation` _returnvalue))
  (:`Pressed`
    (bind _outhit (`KismetSystemLibrary.LineTraceSingle` _returnvalue_2 (+ _returnvalue_2 (* (`self.GetActorForwardVector` _returnvalue) (`self.interactDistance`))) "TraceTypeQuery1"))
    (bind _asinteractable (cast `/Game/Blueprints/Interactable/Interactable` (`.HitActor` (`GameplayStatics.BreakHitResult` _outhit))))
    (`/Game/Blueprints/Interactable/Interactable.OnInteract` _asinteractable)))

(event `InputAction|Watch`
  (params (Key :type "Key Structure" :default "AnyKey"))
  (:`Pressed`
    (bind (_direction _watch_look) (`Timeline|WatchLookAt` :!label _label)
      (:`Update`
        (`SceneComponent.K2_SetRelativeTransform` (`self.Watch_01`) (`KismetMathLibrary.TLerp` (`self.StartTrans`) (`self.EndTrans`) _watch_look) false false))))
  (:`Released`
    (goto _label :!via `Reverse`)))

(fn `UserConstructionScript`
  (set `CharacterMovementComponent.MaxWalkSpeed` (`self.walkSpeed`) (`self.CharacterMovement`))
  (`SceneComponent.K2_SetRelativeTransform` (`self.Watch_01`) (`self.StartTrans`) false false))