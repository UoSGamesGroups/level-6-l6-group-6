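; A locked door Blueprint that animates its Door component from closed to open when the Unlock event fires.
; The construction script caches the door's relative transform as the closed pose, and a timeline lerps from it to OpenTransform.
; Unlock checks IsUnlocked before playing but never sets it here.
; A DebugOpen flag previews the open pose at construction and triggers Unlock on BeginPlay.
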(event `self.ReceiveBeginPlay`
  ;[1 1 1] DEBUG
  (if (`self.DebugOpen`)
    (`self.Event Unlock`)))

(event `Event Unlock`
  (if (not (`self.isUnlocked`))
    (bind (_direction _openalpha) (`Timeline|DoorOpen` :!via `PlayFromStart`)
      (:`Update`
        (`SceneComponent.K2_SetRelativeTransform` (`self.Door`) (`KismetMathLibrary.TLerp` (`self.closeTransform`) (`self.openTransform`) _openalpha) false false)))))

(fn `UserConstructionScript`
  (set `self.closeTransform` (`SceneComponent.GetRelativeTransform` (`self.Door`)))
  ;[1 1 1] Debug
  (if (`self.DebugOpen`)
    (`SceneComponent.K2_SetRelativeTransform` (`self.Door`) (`self.openTransform`) false false)))