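; Generic character Blueprint that provides basic player movement and look controls through axis input events.
; MoveForward and MoveRight add movement input along the actor's forward and right vectors, scaled by the axis value and a MoveSpeed variable.
; Turn and LookUp pass their axis values straight to controller yaw and pitch input.
; BeginPlay, Tick, overlap and the construction script contain no logic.
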(event `InputAxis|MoveForward`
  (params (AxisValue :type "Float (single-precision)"))
  ;[1 1 1] Move
  (`self.AddMovementInput` (`self.GetActorForwardVector`) (* AxisValue (`self.moveSpeed`))))

(event `InputAxis|MoveRight`
  (params (AxisValue :type "Float (single-precision)"))
  ;[1 1 1] Move
  (`self.AddMovementInput` (`self.GetActorRightVector`) (* (`self.moveSpeed`) AxisValue)))

(event `InputAxis|Turn`
  (params (AxisValue :type "Float (single-precision)"))
  (`self.AddControllerYawInput` AxisValue))

(event `InputAxis|LookUp`
  (params (AxisValue :type "Float (single-precision)"))
  (`self.AddControllerPitchInput` AxisValue))

(fn `UserConstructionScript`)